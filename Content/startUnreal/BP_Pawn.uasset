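; BP_Pawn is a basic pawn that moves and looks from player input and prints an elapsed-time clock on screen.
; MoveForward and MoveRight offset the actor along its own vectors without sweep or delta-time scaling.
; Look and lean axes feed controller rotation, with LookUp driving yaw and LookRight driving pitch.
; Tick calls ShowTimeSec, which accumulates delta time and prints minutes:seconds whenever the whole second changes.
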(event EventBeginPlay
  (Development|PrintString "Beginplay"))

(event EventTick
  (params (DeltaSeconds :type Float%20%28single-precision%29))
  (CallFunction|ShowTimeSec DeltaSeconds))

(event Input|ActionEvents|InputActionEnterInput
  (params (Key :type Key%20Structure))
  (:Pressed
    (Development|PrintString "Enter key press")))

(event Input|AxisEvents|InputAxisLookUp
  (params (AxisValue :type Float%20%28single-precision%29))
  (Pawn|Input|AddControllerYawInput AxisValue))

(event Input|AxisEvents|InputAxisLookRight
  (params (AxisValue :type Float%20%28single-precision%29))
  (Pawn|Input|AddControllerPitchInput AxisValue))

(event Input|AxisEvents|InputAxisLean
  (params (AxisValue :type Float%20%28single-precision%29))
  (Pawn|Input|AddControllerRollInput (* AxisValue 1.0)))

(event Input|AxisEvents|InputAxisMoveRight
  (params (AxisValue :type Float%20%28single-precision%29))
  ;[1 1 1] 옆으로의 움직임
  (Transformation|AddActorWorldOffset (* (Transformation|GetActorRightVector) (* AxisValue 1e+01))))

(event Input|AxisEvents|InputAxisMoveForward
  (params (AxisValue :type Float%20%28single-precision%29))
  ;[1 0.2497 0.2696] 앞쪽으로의 움직임
  (Transformation|AddActorWorldOffset (* (Transformation|GetActorForwardVector) (* AxisValue 1e+01))))

(event Input|KeyboardEvents|W
  (params (Key :type Key%20Structure)))

(fn ConstructionScript)

(fn ShowTimeSec
  (params (DeltaSeconds :type Float%20%28single-precision%29))
  (bind _output_get (Variables|Default|SetTotalDeltaSeconds (+ DeltaSeconds (Variables|Default|GetTotalDeltaSeconds))))
  (if (not (== (Variables|Default|GetBeforeInt) (Math|Float|Floor _output_get)))
    (Variables|Default|SetBeforeInt (Math|Float|Floor _output_get))
    (Math|Integer|IncrementInt (Variables|Default|Getsec)
      (:%20%20
        (if (== (Variables|Default|Getsec) 60)
          (Variables|Default|Setsec 0)
          (Math|Integer|IncrementInt (Variables|Default|Getmin)
            (:%20%20
              _)))
        (Development|PrintString (Utilities|String|Append (Utilities|String|Append (Utilities|String|ToString(Integer) (Variables|Default|Getmin)) " : ") (Utilities|String|ToString(Integer) (Variables|Default|Getsec))))))))