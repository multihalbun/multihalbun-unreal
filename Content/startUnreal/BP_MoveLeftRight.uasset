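; BP_MoveLeftRight is an actor that tries to move its Sphere component around a rectangular path.
; Tick uses Right, Up, Left and Down flags as a state machine, adding speed-scaled relative X or Z offsets.
; Turns require exact float equality, vertical legs test Y despite moving Z, and the final leg never re-enables Right.
; An older left-right ping-pong and an empty infinite loop remain unconnected.
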(event EventTick
  (params (DeltaSeconds :type Float%20%28single-precision%29))
  (bind _sphere (Variables|Default|GetSphere))
  (bind _speed (Variables|Default|GetSpeed))
  (bind _returnvalue (* DeltaSeconds _speed))
  (bind _relativelocation (Variables|/Script/Engine.SceneComponent|GetRelativeLocation _sphere))
  (if (Variables|Default|Getright)
    (if (== (.x _relativelocation) 1e+01)
      (Variables|Default|Setright false)
      (Variables|Default|Setup true)
      (else
        (Transformation|AddRelativeLocation _sphere (Math|Vector|MakeVector _returnvalue 0.0 0.0) false false)))
    (elif (Variables|Default|Getup)
      (if (== (.y _relativelocation) 1e+01)
        (Variables|Default|Setup false)
        (Variables|Default|Setleft true)
        (else
          (Transformation|AddRelativeLocation _sphere (Math|Vector|MakeVector 0.0 0.0 _returnvalue) false false)))
      (elif (Variables|Default|Getleft)
        (if (== (.x _relativelocation) 0.0)
          (Variables|Default|Setleft false)
          (Variables|Default|Setdown true)
          (else
            (Transformation|AddRelativeLocation _sphere (Math|Vector|MakeVector (stale _result) 0.0 0.0) false false)))
        (elif (Variables|Default|Getdown)
          (if (== (.y _relativelocation) 0.0)
            (Variables|Default|Setdown false)
            (Variables|Default|Setright false)
            (else
              (Transformation|AddRelativeLocation _sphere (Math|Vector|MakeVector 0.0 0.0 (stale _result)) false false))))))))

(fn ConstructionScript)